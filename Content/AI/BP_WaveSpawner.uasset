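; BP_WaveSpawner spawns escalating waves of zombie characters on a repeating timer.
; BeginPlay starts a looping timer, so the first wave arrives after one full interval of a few minutes.
; Each wave permanently raises BaseToSpawn by a random amount, then uses it as the spawn loop bound.
; Every zombie spawns at a randomly picked HordeLocations actor transform, adjusting for collisions but always spawning.
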(event `self.ReceiveBeginPlay`
  (`KismetSystemLibrary.K2_SetTimerDelegate` (delegate `Spawn wave`) 220.0 true))

(event `Spawn wave`
  (bind _horde_locations (`self.Horde Locations`))
  (bind _output_get (set `self.Base to Spawn` (+ (`self.Base to Spawn`) (`KismetMathLibrary.RandomIntegerInRange` 5 10))))
  (for _ (range (+ _output_get 1))
    (`|SpawnActorFromClass` "/Game/AI/ZombieCharacter.ZombieCharacter_C" (`self.GetTransform` (`|GetArrayItem` _horde_locations (`KismetMathLibrary.RandomInteger` (`KismetArrayLibrary.Array_Length` _horde_locations)))) "AdjustIfPossibleButAlwaysSpawn" "MultiplyWithRoot" null null)))

(fn `UserConstructionScript`)