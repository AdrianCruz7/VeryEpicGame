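; Meteor spawner that periodically launches a meteor aimed at the first player character.
; A looping timer from BeginPlay spawns a temporary spot actor at a random horizontal position and fixed height.
; The spot rotates toward the player's current location, lends its transform to a new BP_Meteor, then is destroyed.
; A SimpleMoveToActor call targets the new meteor, with no controller specified.
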(event `self.ReceiveBeginPlay`
  (`KismetSystemLibrary.K2_SetTimerDelegate` (delegate `TryMeteor`) 73.0 true))

(event `TryMeteor`
  (bind _returnvalue (`self.K2_GetActorLocation` (`GameplayStatics.GetPlayerCharacter` 0)))
  (bind _returnvalue_2 (`|SpawnActorFromClass` "/Game/AI/BP_MeteorSpot.BP_MeteorSpot_C" (`KismetMathLibrary.MakeTransform` (`KismetMathLibrary.MakeVector` (`KismetMathLibrary.Conv_IntToDouble` (`KismetMathLibrary.RandomIntegerInRange` -15000 15000)) (`KismetMathLibrary.Conv_IntToDouble` (`KismetMathLibrary.RandomIntegerInRange` -15000 15000)) 3500.0)) "Undefined" "MultiplyWithRoot" null null))
  (bind _returnvalue_3 (`self.GetTransform` _returnvalue_2))
  (bind (_returnvalue_location _returnvalue_rotation) (`KismetMathLibrary.BreakTransform` (`KismetAnimationLibrary.K2_LookAt` _returnvalue_3 _returnvalue _returnvalue)))
  (`self.K2_SetActorRotation` _returnvalue_2 _returnvalue_rotation false)
  (bind _returnvalue_4 (`|SpawnActorFromClass` "/Game/AI/BP_Meteor.BP_Meteor_C" _returnvalue_3 "Undefined" "MultiplyWithRoot" null null))
  (`AIBlueprintHelperLibrary.SimpleMoveToActor` null _returnvalue_4)
  (`self.K2_DestroyActor` _returnvalue_2))

(fn `UserConstructionScript`)