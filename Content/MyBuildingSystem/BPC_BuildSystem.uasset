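; Player pawn component that runs a build mode preview, toggled on and off with the B key.
; While active, it line traces each tick from the pawn's camera out to BuildRange on the Visibility channel.
; The first hit creates a static mesh component on the pawn, and each hit moves it to the impact location with zero rotation.
; It assigns no mesh and has no placement or preview removal logic.
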(event `self.ReceiveTick`
  (params (DeltaSeconds :type "Float (single-precision)"))
  (if (`self.InBuildMode`)
    (`self.Preview Loop`)))

(event `self.ReceiveBeginPlay`
  (bind _asplayer_pawn (cast `/Game/Player/PlayerPawn` (`self.GetOwner`)))
  (set `self.Player` _asplayer_pawn)
  (set `self.Camera` (`/Game/Player/PlayerPawn.Camera` _asplayer_pawn)))

(event `Preview Loop`
  (bind (_returnvalue_location _returnvalue_rotation) (`KismetMathLibrary.BreakTransform` (`SceneComponent.K2_GetComponentToWorld` (`self.Camera`))))
  (`/Engine/EditorBlueprintResources/StandardMacros.IsValid` (`self.Camera`)
    (:`Is Valid`
      _)
    (:`Is Not Valid`
      (set `self.Camera` (`/Game/Player/PlayerPawn.Camera` (`self.Player`)))))
  (bind (_outhit _returnvalue) (`KismetSystemLibrary.LineTraceSingle` _returnvalue_location (+ _returnvalue_location (* (`KismetMathLibrary.GetForwardVector` _returnvalue_rotation) (`self.Build Range`))) "TraceTypeQuery1"))
  (if _returnvalue
    (`|ExecutionSequence`
      (:`then_0`
        (`/Engine/EditorBlueprintResources/StandardMacros.DoOnce` false
          (:`Completed`
            (bind _returnvalue_2 (`|AddComponentByClass` (`self.Player`) "/Script/Engine.StaticMeshComponent" false (`self.Build Preview Transform`)))
            (set `self.Preview Mesh` _returnvalue_2))))
      (:`then_1`
        (bind _output_get (set `self.Build Preview Transform` (`KismetMathLibrary.MakeTransform` (`.Location` (`GameplayStatics.BreakHitResult` _outhit)))))
        (`SceneComponent.K2_SetWorldTransform` (`self.Preview Mesh`) _output_get false false)))))

(event `Key|B`
  (params (Key :type "Key Structure"))
  (:`Pressed`
    (`/Engine/EditorBlueprintResources/StandardMacros.FlipFlop`
      (:`A`
        (set `self.InBuildMode` true))
      (:`B`
        (set `self.InBuildMode` false)))))

(event `Key|J`
  (params (Key :type "Key Structure")))